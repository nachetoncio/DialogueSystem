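; BP_NPC is an interactable dialogue character that runs its conversations as a Behavior Tree on its AI controller.
; Interact starts the player's dialogue camera and HUD, aims its spring-arm camera and turns the NPC toward the player via timeline; repeat interactions advance dialogue.
; Dispatchers relay continue and choice events, Speak updates the player's dialogue display, and FinishInteract stops the tree.
; Tick also line-traces forward, messaging any interactable hit.
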(event EventTick
  (params (DeltaSeconds :type Float%20%28single-precision%29))
  (bind _returnvalue (Transformation|GetActorLocation))
  (bind (_outhit _returnvalue_2) (Collision|LineTraceByChannel _returnvalue (+ _returnvalue (* (Transformation|GetActorForwardVector) (Variables|Default|GetInteractableCheckRayDistance))) "TraceTypeQuery1" false 0 "None"))
  (if _returnvalue_2
    (if (Utilities|DoesObjectImplementInterface (.HitActor (Collision|BreakHitResult _outhit)) "/Game/DialogueSystem/Blueprints/Interfaces/BI_Interactable.BI_Interactable_C")
      (Class|BIInteractable|Interact(Message) (.HitActor (Collision|BreakHitResult _outhit)))
      (CallFunction|GetInteractableName (Variables|Default|GetCharacterName)))))

(event EventInteract
  (params (PlayerRef :type Actor%20Object%20Reference))
  ;[0.9094 0.4391 0.1511] Event Interact
  (Variables|Default|SetPlayer%20Ref PlayerRef)
  (if (not (Variables|Default|GetDialogueStarted))
    (Variables|Default|SetDialogueStarted true)
    (CallFunction|SetDialogueCameraLookatPlayer (Variables|Default|GetPlayer%20Ref))
    (Class|BIDialogablePlayer|InitDialogueCamera(Message) (Variables|Default|GetPlayer%20Ref))
    (Class|BIDialogablePlayer|InitDialogueHUD(Message) (Variables|Default|GetPlayer%20Ref) (Variables|Default|GetCharacterName))
    (AI|RunBehaviorTree (AI|GetAIController self) (Variables|Default|GetDialogueTree))
    (Variables|Default|SetPreDialogueNpcRotation (Transformation|GetActorRotation))
    (bind _t_dialoguerotation (Timeline|T_SetDialogueRotation PlayFromStart)
      (:Update
        (Transformation|SetActorRotation (Math|Rotator|Lerp(Rotator) (Variables|Default|GetPreDialogueNpcRotation) (Pawn|GetDesiredRotation (Variables|Default|GetPlayer%20Ref)) _t_dialoguerotation true))))
    (else
      (CallFunction|AdvanceDialogue))))

(event EventMoveto
  (params (TargetLocation :type Vector :default "0, 0, 0"))
  ;[0.7219 0.2559 0.6176] Event Move To
  (AI|AIMoveTo self TargetLocation 0 5.0 false))

(event EventFinishInteract
  (params (PlayerRef :type Actor%20Object%20Reference))
  ;[0.9177 0.2985 0.7629] Event Finish Interact
  (Variables|Default|SetDialogueStarted false)
  (Class|BIDialogablePlayer|FinishDialogue(Message) PlayerRef)
  (AI|Logic|StopLogic (Variables|/Script/AIModule.AIController|GetBrainComponent (AI|GetAIController self)) "Dialogue Finished"))

(event EventSelectChoice
  (params (ChoiceIndex :type Integer))
  ;[1 0.2684 0.5398] Event SelectChoice to Dispatcher OnSelectChoice
  (Default|CallOnSelectChoice ChoiceIndex))

(event EventSetDialogueTree
  (params (BehaviorTree :type Behavior%20Tree%20Object%20Reference))
  ;[0.6635 0.2152 0.5291] Event Set Dialogue Tree
  (Variables|Default|SetDialogueTree BehaviorTree))

(fn ConstructionScript
  ;[1 1 1] Construction Script
  (Variables|/Script/Engine.SpringArmComponent|SetTargetArmLength (Variables|Default|GetSpringArm) (Variables|Default|GetDialogueCameraArmLength))
  (Utilities|Struct|SetmembersinCameraFocusSettings (Variables|/Script/CinematicCamera.CineCameraComponent|GetFocusSettings (Variables|Default|GetDialogueCamera)) (Variables|/Script/Engine.SpringArmComponent|GetTargetArmLength (Variables|Default|GetSpringArm)))
  (Transformation|SetWorldRotation (Variables|Default|GetSpringArm) (Math|Rotator|MakeRotator 0.0 0.0 (.yaw (Math|Rotator|MakeRotfromZ (Transformation|GetActorRightVector)))) false false))

(fn SetDialogueCameraLookatPlayer
  (params (PlayerRef :type Actor%20Object%20Reference))
  ;[0.01 0.01 0.01] Set Dialogue Camera Look at Player
  (Transformation|SetWorldRotation (Variables|Default|GetSpringArm) (Math|Rotator|MakeRotator 0.0 0.0 (.yaw (Math|Rotator|FindLookatRotation (Transformation|GetActorLocation PlayerRef) (Transformation|GetActorLocation)))) false false))

(fn AdvanceDialogue
  ;[0.01 0.01 0.01] Advance Dialogue
  (Default|CallOnContinueDialogue))

(fn Speak
  (params (Sentence :type Text))
  ;[1 0.5496 0.6236] Speak
  (Class|BIDialogablePlayer|UpdateDialogueInfo(Message) (Variables|Default|GetPlayer%20Ref) Sentence))

(fn GetHeadTransform
  (return (Transformation|GetSocketTransform (Variables|Character|GetMesh) (Variables|Default|GetHeadName) "RTS_World")))

(fn GetInteractableName
  (params (Name :type Text))
  (return ""))